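; Dungeon game mode that tracks the player's score and the win and loss state of a match.
; BeginPlay resets the state and sets the score target, and AddScore accumulates points until that target triggers HandleVictory.
; HandleVictory and HandleDefeat set their flags, print Spanish debug messages and call Win or Defeat, apparently event dispatchers.
; Nothing in this Blueprint invokes HandleDefeat or guards against repeated victory calls.
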(event EventBeginPlay
  (Variables|Default|SetPlayerScore 0)
  (Variables|Default|SetbGameOver false)
  (Variables|Default|SetbVictory false)
  (Variables|Default|SetNeededScore 100))

(fn ConstructionScript)

(fn AddScore
  (params (Ammount :type Integer))
  ;[0.15 0.15 0.15 0.5] AddScore
  (bind _output_get (Variables|Default|SetPlayerScore (+ Ammount (Variables|Default|GetPlayerScore))))
  (if (>= _output_get (Variables|Default|GetNeededScore))
    (CallFunction|HandleVictory)
    (else
      (Development|PrintString "Nuevo Puntaje:")
      (Development|PrintString (Utilities|String|ToString(Integer) (Variables|Default|GetPlayerScore))))))

(fn HandleVictory
  ;[0.15 0.15 0.15 0.5] HandleVictory - Aca va la logica al haber ganado
  (Variables|Default|SetbVictory true)
  (Development|PrintString "Has Ganado!")
  (Default|CallWin))

(fn HandleDefeat
  ;[0.15 0.15 0.15 0.5] HandleDefeat - Logica al perder
  (Variables|Default|SetbGameOver true)
  (Development|PrintString "Perdiste")
  (Default|CallDefeat))