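; Slime enemy for the dungeon game that chases the player and attacks with leaps.
; An event-driven state machine uses sight and attack-range spheres to switch between idle, AI MoveTo chasing with timed retries, launched leaps and timed cooldown.
; Its damage sphere hurts the player's health component, throttled by a timer.
; Player hits lower its health bar behind a brief invulnerability window, and death adds score through the game mode.
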(event OnComponentBeginOverlap(SightSphere)
  (params (OverlappedComponent :type Primitive%20Component%20Object%20Reference) (OtherActor :type Actor%20Object%20Reference) (OtherComp :type Primitive%20Component%20Object%20Reference) (OtherBodyIndex :type Integer) (bFromSweep :type Boolean) (SweepResult :type Hit%20Result%20Structure%20%28by%20ref%29))
  ;[0.15 0.15 0.15 0.5] SightSphereOverlap
  (if (== OtherActor (Game|Player|GetPlayerPawn 0))
    (Variables|Default|SetTargetPlayer OtherActor)
    (CallFunction|SetState "NewEnumerator1")))

(event OnComponentEndOverlap(SightSphere)
  (params (OverlappedComponent :type Primitive%20Component%20Object%20Reference) (OtherActor :type Actor%20Object%20Reference) (OtherComp :type Primitive%20Component%20Object%20Reference) (OtherBodyIndex :type Integer))
  ;[0.15 0.15 0.15 0.5] SightSphereOverlap
  (if (== OtherActor (Variables|Default|GetTargetPlayer))
    (Variables|Default|SetTargetPlayer 0)
    (CallFunction|SetState "NewEnumerator0")))

(event OnComponentBeginOverlap(AttackRangeSphere)
  (params (OverlappedComponent :type Primitive%20Component%20Object%20Reference) (OtherActor :type Actor%20Object%20Reference) (OtherComp :type Primitive%20Component%20Object%20Reference) (OtherBodyIndex :type Integer) (bFromSweep :type Boolean) (SweepResult :type Hit%20Result%20Structure%20%28by%20ref%29))
  ;[0.15 0.15 0.15 0.5] AttackRangeSphereOverlap
  (if (== OtherActor (Game|Player|GetPlayerPawn 0))
    (if (Variables|Default|GetbCanAttack)
      (CallFunction|SetState "NewEnumerator2"))))

(event OnComponentEndOverlap(AttackRangeSphere)
  (params (OverlappedComponent :type Primitive%20Component%20Object%20Reference) (OtherActor :type Actor%20Object%20Reference) (OtherComp :type Primitive%20Component%20Object%20Reference) (OtherBodyIndex :type Integer))
  ;[0.15 0.15 0.15 0.5] AttackRangeSphereOverlap
  (if (== OtherActor (Variables|Default|GetTargetPlayer))
    (if (!= (Variables|Default|GetCurrentState) 2)
      (CallFunction|SetState "NewEnumerator1"))))

(event OnComponentBeginOverlap(DamageSphere)
  (params (OverlappedComponent :type Primitive%20Component%20Object%20Reference) (OtherActor :type Actor%20Object%20Reference) (OtherComp :type Primitive%20Component%20Object%20Reference) (OtherBodyIndex :type Integer) (bFromSweep :type Boolean) (SweepResult :type Hit%20Result%20Structure%20%28by%20ref%29))
  (bind _targetplayer (Variables|Default|GetTargetPlayer))
  (if (Variables|Default|GetbCanTouchDamage)
    (Development|PrintString "HIT")
    (if (== OtherActor _targetplayer)
      (bind _asbp_duplicated_third_person_character_1 (Utilities|Casting|CastToBP_DuplicatedThirdPersonCharacter1 _targetplayer))
      (Utilities|IsValid (Actor|GetComponentbyClass _asbp_duplicated_third_person_character_1 "/Game/Assets/3D/Blueprints/BPC_HealthSystemCoponent.BPC_HealthSystemCoponent_C")
        (:Is%20Valid
          (Class|HealthSystemComponent|ReceiveDamage (Actor|GetComponentbyClass _asbp_duplicated_third_person_character_1 "/Game/Assets/3D/Blueprints/BPC_HealthSystemCoponent.BPC_HealthSystemCoponent_C"))
          (Development|PrintString "daño recibido de slime")
          (Variables|Default|SetbCanTouchDamage false)
          (Utilities|Time|SetTimerbyFunctionName 0 "ResetTouchDamage" 1.0))))))

(event Custom|UpdateState
  (bind _targetplayer (Variables|Default|GetTargetPlayer))
  (bind _returnvalue (Utilities|IsValid _targetplayer))
  ;[0.15 0.15 0.15 0.5] UpdateState
  (switch Utilities|FlowControl|Switch|SwitchonESlimeState (Variables|Default|GetCurrentState)
    (:NewEnumerator0
      (if _returnvalue
        (CallFunction|SetState "NewEnumerator1")))
    (:NewEnumerator1
      (if _returnvalue
        (if (Collision|IsOverlappingActor (Variables|Default|GetAttackRangeSphere) (Variables|Default|GetTargetPlayer) :!class /Script/Engine.PrimitiveComponent)
          (if (Variables|Default|GetbCanAttack)
            (CallFunction|SetState "NewEnumerator2")
            (else
              (CallFunction|StartChasing :!label _label)))
          (else
            (goto _label)))
        (else
          (CallFunction|SetState "NewEnumerator0"))))))

(event Custom|SetState
  (params (NewState :type ESlimeState%20Enum :default "NewEnumerator0"))
  ;[0.15 0.15 0.15 0.5] SetState
  (bind _output_get (Variables|Default|SetCurrentState NewState))
  (switch Utilities|FlowControl|Switch|SwitchonESlimeState _output_get
    (:NewEnumerator0
      (Class|NavMovementInterface|StopActiveMovement (Variables|Character|GetCharacterMovement)))
    (:NewEnumerator1
      (CallFunction|StartChasing))
    (:NewEnumerator2
      (CallFunction|DoLeapAttack))))

(event Custom|StartChasing
  ;[0.15 0.15 0.15 0.5] StartChasing
  (if (Utilities|IsValid (Variables|Default|GetTargetPlayer))
    (Development|PrintString "Empezando a perseguir")
    (AI|AIMoveTo self "0, 0, 0" (Variables|Default|GetTargetPlayer) (Variables|Default|GetChaseAcceptRadius) true
      (:OnSuccess
        (Utilities|Time|SetTimerbyFunctionName 0 "RetryMoveTo" 0.5))
      (:OnFail
        (Utilities|Time|SetTimerbyFunctionName 0 "RetryMoveTo" 0.8)))))

(event Custom|DoLeapAttack
  (bind _returnvalue (Transformation|GetActorLocation))
  (bind _leaphorizontalpower (Variables|Default|GetLeapHorizontalPower))
  (bind _targetplayer (Variables|Default|GetTargetPlayer))
  (bind _returnvalue_2 (Transformation|GetActorLocation _targetplayer))
  (bind _returnvalue_3 (- _returnvalue_2 _returnvalue))
  (bind _returnvalue_4 (Math|Vector|Normalize _returnvalue_3))
  (bind (_x _y) (Math|Vector|BreakVector _returnvalue_4))
  ;[0.15 0.15 0.15 0.5] DoLeapAttack
  (Variables|Default|SetbCanAttack true)
  (Character|LaunchCharacter (Math|Vector|MakeVector (* _x _leaphorizontalpower) (* _y _leaphorizontalpower) (Variables|Default|GetLeapVerticalPower)) true true)
  (CallFunction|SetState "NewEnumerator3")
  (Utilities|Time|SetTimerbyFunctionName 0 "EndAttackCooldown" (Variables|Default|GetAttackCooldown)))

(event Custom|EndAttackCooldown
  ;[0.15 0.15 0.15 0.5] EndAttackCooldown
  (Variables|Default|SetbCanAttack true)
  (if (Utilities|IsValid (Variables|Default|GetTargetPlayer))
    (if (Collision|IsOverlappingActor (Variables|Default|GetAttackRangeSphere) (Variables|Default|GetTargetPlayer) :!class /Script/Engine.PrimitiveComponent)
      (CallFunction|SetState "NewEnumerator2")
      (else
        (CallFunction|SetState "NewEnumerator1")))
    (else
      (CallFunction|SetState "NewEnumerator1"))))

(event Custom|RetryMoveTo
  ;[0.15 0.15 0.15 0.5] RetryMoveTo
  (if (!= (Variables|Default|GetCurrentState) 2)
    (CallFunction|StartChasing)))

(event Custom|HitByPlayer
  ;[0.15 0.15 0.15 0.5] GetHit
  (if (Variables|Default|GetbCanReceiveDamage)
    (Variables|Default|SetHealth (- (Variables|Default|GetHealth) 4e+01))
    (if (<= (Variables|Default|GetHealth) 0.0)
      (bind _asbp_game_mode_dungeon (Utilities|Casting|CastToBP_GameMode_Dungeon (Game|GetGameMode))
        (:then
          (Default|AddScore _asbp_game_mode_dungeon 50)
          (Actor|DestroyActor))
        (:CastFailed
          (Development|PrintString "Failed")))
      (else
        (bind _aswbp_enemy_health (Utilities|Casting|CastToWBP_EnemyHealth (UserInterface|GetUserWidgetObject (Variables|Default|GetHealthBarWidget))))
        (Variables|Default|SetAs%20WBP%20Enemy%20Health _aswbp_enemy_health)
        (Variables|/Game/Assets/3D/Widget/WBP_EnemyHealth.WBP_EnemyHealth_C|SetHealth (Variables|Default|GetAs%20WBP%20Enemy%20Health) (/ (Variables|Default|GetHealth) 1e+02))
        (Variables|Default|SetbCanReceiveDamage false)
        (Utilities|Time|SetTimerbyFunctionName 0 "ResetDamageFlag" 0.2)))))

(event Custom|ResetDamageFlag
  (Variables|Default|SetbCanReceiveDamage true))

(event Custom|ResetTouchDamage
  (Variables|Default|SetbCanTouchDamage true))

(event EventBeginPlay
  (Variables|Default|SetCurrentState "NewEnumerator0")
  (Variables|Default|SetAttackCooldown 2.0)
  (Variables|Default|SetbCanAttack true)
  (Variables|Default|SetLeapHorizontalPower 8e+02)
  (Variables|Default|SetLeapVerticalPower 6e+02)
  (Variables|Default|SetChaseAcceptRadius 1.2e+02)
  (Variables|Default|SetHealth 1e+02)
  (bind _aswbp_enemy_health (Utilities|Casting|CastToWBP_EnemyHealth (UserInterface|GetUserWidgetObject (Variables|Default|GetHealthBarWidget))))
  (Variables|Default|SetAs%20WBP%20Enemy%20Health _aswbp_enemy_health)
  (Variables|/Game/Assets/3D/Widget/WBP_EnemyHealth.WBP_EnemyHealth_C|SetHealth (Variables|Default|GetAs%20WBP%20Enemy%20Health) (/ (Variables|Default|GetHealth) 1e+02))
  (Variables|Default|SetbCanReceiveDamage true)
  (Variables|Default|SetbCanTouchDamage true))

(fn ConstructionScript)