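; Inventory component that keeps a list of item names in an Items array.
; AddItem appends a name, while RemoveItem does nothing because its Remove node is not connected.
; HasItem loops through the array and returns true on the first match, otherwise returning the same element comparison after the loop.
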(event Custom|AddItem
  (params (ItemName :type Name))
  ;[0.15 0.15 0.15 0.5] Add/RemoveItem
  (Utilities|Array|Add (Variables|Default|GetItems) ItemName))

(event Custom|RemoveItem
  (params (ItemName :type Name))
  ;[0.15 0.15 0.15 0.5] Add/RemoveItem
)

(event EventBeginPlay)

(fn HasItem
  (params (ItemName :type Name))
  ;[0.15 0.15 0.15 0.5] HasItem
  (for _array_element (Variables|Default|GetItems)
    (if (== _array_element ItemName)
      (return (== _array_element ItemName))))
  (return (== _array_element ItemName)))