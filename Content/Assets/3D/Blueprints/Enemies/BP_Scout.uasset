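; Scout enemy for the dungeon that carries a horn and blows it as its attack.
; Loads stats from DT_EnemyStats and exposes patrol route, speed tiers and looping escape-point movement, alongside a hand-socket sphere trace that hits the player.
; Player hits update a health bar behind a brief invulnerability timer.
; Death awards score through BP_GameMode_Dungeon, ragdolls the mesh, notifies AIC_EnemyScout and unpossesses it.
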(event Custom|Die
  (bind _mesh (Variables|Character|GetMesh))
  (Collision|SetCollisionProfileName _mesh "Ragdoll" true :!class /Script/Engine.PrimitiveComponent)
  (Physics|SetSimulatePhysics _mesh true)
  (Components|DestroyComponent (Variables|Default|GetHealthBarWidget))
  (bind _asaic_enemy_scout (Utilities|Casting|CastToAIC_EnemyScout (Pawn|GetController)))
  (Default|HandleDead _asaic_enemy_scout self)
  (Audio|PlaySoundatLocation "/Game/Assets/3D/Sounds/SFX/Die.Die" "0, 0, 0" "0, 0, 0" 1.0 1.0 0.0 0 0 0 0)
  (Pawn|UnPossess _asaic_enemy_scout))

(event Custom|ResetDamageFlag
  (Variables|Default|SetCan%20Receive%20Damage true))

(event Custom|Attack
  (Animation|Montage|PlayMontage (Variables|Character|GetMesh) "/Game/Assets/3D/Animation/Scout/AN_PlayHorn.AN_PlayHorn"
    (:then
      (Audio|PlaySoundatLocation "/Game/Assets/3D/Sounds/SFX/Horn.Horn" "0, 0, 0" "0, 0, 0" 1.0 1.0 0.0 0 0 0 0))
    (:OnCompleted
      (Default|CallOnAttackEnd :!label _label))
    (:OnInterrupted
      (goto _label))))

(event Custom|WieldHorn
  (bind _returnvalue (Game|SpawnActorfromClass "/Game/Assets/3D/Weapons/BP_Horn.BP_Horn_C" (Transformation|GetActorTransform) "Undefined" "MultiplyWithRoot" 0 0))
  (Transformation|AttachComponentToComponent _returnvalue (Variables|Character|GetMesh) "hand_r_Horn_Socket" "SnapToTarget" "SnapToTarget" "SnapToTarget" true))

(event Custom|Focus
  (bind _returnvalue (Actor|GetActorOfClass "/Game/Assets/3D/Blueprints/Enemies/AI/AIC_EnemyBase.AIC_EnemyBase_C"))
  (bind _asbp_duplicated_third_person_character_1 (Utilities|Casting|CastToBP_DuplicatedThirdPersonCharacter1 (Class|CharacterMovementComponent|GetCharacterOwner (Variables|Character|GetCharacterMovement))))
  (AI|SetFocus _returnvalue _asbp_duplicated_third_person_character_1))

(event Custom|Escape
  (AI|AIMoveTo self "0, 0, 0" (Utilities|Array|Get(acopy) (Variables|Default|GetEscapePoints) (Variables|Default|GetCurrentWaypoint)) 0.0 false
    (:then
      (Math|Integer|IncrementInt (Variables|Default|GetCurrentWaypoint)
        (:%20%20
          (if (>= (Variables|Default|GetCurrentWaypoint) (Utilities|Array|Length (Variables|Default|GetEscapePoints)))
            (Variables|Default|SetCurrentWaypoint 0)))))))

(event Custom|HitByPlayer
  ;[0.15 0.15 0.15 0.5] GetHit
  (if (Variables|Default|GetCan%20Receive%20Damage)
    (Variables|Default|SetHealth (- (Variables|Default|GetHealth) (.DamageRecieved (Utilities|Struct|BreakST_EnemyStats (Variables|Default|GetStats)))))
    (if (<= (Variables|Default|GetHealth) 0.0)
      (bind _asbp_game_mode_dungeon (Utilities|Casting|CastToBP_GameMode_Dungeon (Game|GetGameMode))
        (:then
          (Default|AddScore _asbp_game_mode_dungeon 50)
          (Collision|SetCollisionProfileName (Variables|Collision|GetCapsuleComponent) (Utilities|Name|MakeLiteralName "NoCollision") true :!class /Script/Engine.PrimitiveComponent)
          (CallFunction|Die))
        (:CastFailed
          (Development|PrintString "Failed")))
      (else
        (bind _aswbp_enemy_health (Utilities|Casting|CastToWBP_EnemyHealth (UserInterface|GetUserWidgetObject (Variables|Default|GetHealthBarWidget))))
        (Variables|Default|SetAs%20WBP%20Enemy%20Health _aswbp_enemy_health)
        (Variables|/Game/Assets/3D/Widget/WBP_EnemyHealth.WBP_EnemyHealth_C|SetHealth (Variables|Default|GetAs%20WBP%20Enemy%20Health) (/ (Variables|Default|GetHealth) (.MaxHealth (Utilities|Struct|BreakST_EnemyStats (Variables|Default|GetStats)))))
        (Variables|Default|SetCan%20Receive%20Damage false)
        (Utilities|Time|SetTimerbyFunctionName 0 "ResetDamageFlag" 0.2)))))

(event EventBeginPlay
  (CallFunction|WieldHorn)
  (Variables|Default|SetCan%20Receive%20Damage true)
  (bind _returnvalue (Utilities|GetDataTableRow "/Game/Assets/3D/Struct/DT_EnemyStats.DT_EnemyStats" (Variables|Default|GetEnemyRowName))
    (:then
      (if true
        (bind _output_get (Variables|Default|SetStats _returnvalue))
        (Variables|Default|SetHealth (.MaxHealth (Utilities|Struct|BreakST_EnemyStats _output_get)))
        (bind _aswbp_enemy_health (Utilities|Casting|CastToWBP_EnemyHealth (UserInterface|GetUserWidgetObject (Variables|Default|GetHealthBarWidget))))
        (Variables|Default|SetAs%20WBP%20Enemy%20Health _aswbp_enemy_health)
        (Variables|/Game/Assets/3D/Widget/WBP_EnemyHealth.WBP_EnemyHealth_C|SetHealth (Variables|Default|GetAs%20WBP%20Enemy%20Health) (/ (Variables|Default|GetHealth) (.MaxHealth (Utilities|Struct|BreakST_EnemyStats _output_get))))))))

(fn ConstructionScript)

(fn AIHitDetect
  (bind _mesh (Variables|Character|GetMesh))
  (bind _returnvalue (Transformation|GetSocketLocation _mesh "hand_r_sword_socket"))
  (bind _outhit (Collision|SphereTraceForObjects _returnvalue _returnvalue 5e+01 (Utilities|Array|MakeArray "ObjectTypeQuery3") false 0 "ForDuration"))
  (bind _asbp_duplicated_third_person_character_1 (Utilities|Casting|CastToBP_DuplicatedThirdPersonCharacter1 (.HitActor (Collision|BreakHitResult _outhit))))
  (Default|GetHit _asbp_duplicated_third_person_character_1))

(fn GetPatrolRoute
  (return (Variables|AI|GetPatrolRoute)))

(fn SetMovementSpeed
  (params (Speed :type E_MovementSpeed%20Enum :default "NewEnumerator0"))
  (bind _output_get (Variables|/Script/Engine.CharacterMovementComponent|SetMaxWalkSpeed (Variables|Character|GetCharacterMovement) (Utilities|Select :Index Speed :NewEnumerator0 0.0 :NewEnumerator1 3e+02 :NewEnumerator2 4.5e+02 :NewEnumerator3 6e+02)))
  (return _output_get))