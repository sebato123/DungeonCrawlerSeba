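; Dungeon enemy character that wields a spawned sword, shows a health bar and awards score when the player kills it.
; Player hits reduce health behind a short invulnerability timer; death disables capsule collision, ragdolls the mesh and removes the bar.
; Attack plays a montage and signals its end, while AIHitDetect sphere-traces at the sword-hand socket to damage the player.
; It also exposes patrol route, speed presets and a focus event for AI.
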(event Custom|Die
  (bind _mesh (Variables|Character|GetMesh))
  (Collision|SetCollisionProfileName _mesh "Ragdoll" true :!class /Script/Engine.PrimitiveComponent)
  (Physics|SetSimulatePhysics _mesh true)
  (Components|DestroyComponent (Variables|Default|GetHealthBarWidget)))

(event Custom|ResetDamageFlag
  (Variables|Default|SetCan%20Receive%20Damage true))

(event Custom|Attack
  (Animation|Montage|PlayMontage (Variables|Character|GetMesh) "/Game/Assets/3D/Animation/Enemy/AM_ATK1.AM_ATK1"
    (:OnCompleted
      _)
    (:OnInterrupted
      _))
  (Default|CallOnAttackEnd))

(event Custom|WieldSword
  (bind _returnvalue (Game|SpawnActorfromClass "/Game/Assets/3D/Weapons/BP_Sword.BP_Sword_C" (Transformation|GetActorTransform) "Undefined" "MultiplyWithRoot" 0 0))
  (Transformation|AttachComponentToComponent _returnvalue (Variables|Character|GetMesh) "hand_r_sword_socket" "SnapToTarget" "SnapToTarget" "SnapToTarget" true))

(event Custom|Focus
  (bind _returnvalue (Actor|GetActorOfClass "/Game/Assets/3D/Blueprints/Enemies/AI/AIC_EnemyBase.AIC_EnemyBase_C"))
  (bind _asbp_duplicated_third_person_character_1 (Utilities|Casting|CastToBP_DuplicatedThirdPersonCharacter1 (Class|CharacterMovementComponent|GetCharacterOwner (Variables|Character|GetCharacterMovement))))
  (AI|SetFocus _returnvalue _asbp_duplicated_third_person_character_1))

(event Custom|HitByPlayer
  ;[0.15 0.15 0.15 0.5] GetHit
  (if (Variables|Default|GetCan%20Receive%20Damage)
    (Variables|Default|SetHealth (- (Variables|Default|GetHealth) 4e+01))
    (if (<= (Variables|Default|GetHealth) 0.0)
      (bind _asbp_game_mode_dungeon (Utilities|Casting|CastToBP_GameMode_Dungeon (Game|GetGameMode))
        (:then
          (Default|AddScore _asbp_game_mode_dungeon 50)
          (Collision|SetCollisionProfileName (Variables|Collision|GetCapsuleComponent) (Utilities|Name|MakeLiteralName "NoCollision") true :!class /Script/Engine.PrimitiveComponent)
          (CallFunction|Die))
        (:CastFailed
          (Development|PrintString "Failed")))
      (else
        (bind _aswbp_enemy_health (Utilities|Casting|CastToWBP_EnemyHealth (UserInterface|GetUserWidgetObject (Variables|Default|GetHealthBarWidget))))
        (Variables|Default|SetAs%20WBP%20Enemy%20Health _aswbp_enemy_health)
        (Variables|/Game/Assets/3D/Widget/WBP_EnemyHealth.WBP_EnemyHealth_C|SetHealth (Variables|Default|GetAs%20WBP%20Enemy%20Health) (/ (Variables|Default|GetHealth) 1e+02))
        (Variables|Default|SetCan%20Receive%20Damage false)
        (Utilities|Time|SetTimerbyFunctionName 0 "ResetDamageFlag" 0.2)))))

(event EventBeginPlay
  (CallFunction|WieldSword)
  (Variables|Default|SetCan%20Receive%20Damage true)
  (Variables|Default|SetHealth 1e+02)
  (bind _aswbp_enemy_health (Utilities|Casting|CastToWBP_EnemyHealth (UserInterface|GetUserWidgetObject (Variables|Default|GetHealthBarWidget))))
  (Variables|Default|SetAs%20WBP%20Enemy%20Health _aswbp_enemy_health)
  (Variables|/Game/Assets/3D/Widget/WBP_EnemyHealth.WBP_EnemyHealth_C|SetHealth (Variables|Default|GetAs%20WBP%20Enemy%20Health) (/ (Variables|Default|GetHealth) 1e+02)))

(event Collision|EventActorBeginOverlap
  (params (OtherActor :type Actor%20Object%20Reference)))

(event EventTick
  (params (DeltaSeconds :type Float%20%28single-precision%29)))

(fn ConstructionScript)

(fn AIHitDetect
  (bind _mesh (Variables|Character|GetMesh))
  (bind _returnvalue (Transformation|GetSocketLocation _mesh "hand_r_sword_socket"))
  (bind _outhit (Collision|SphereTraceForObjects _returnvalue _returnvalue 5e+01 (Utilities|Array|MakeArray "ObjectTypeQuery3") false 0 "ForDuration"))
  (bind _asbp_duplicated_third_person_character_1 (Utilities|Casting|CastToBP_DuplicatedThirdPersonCharacter1 (.HitActor (Collision|BreakHitResult _outhit))))
  (Default|GetHit _asbp_duplicated_third_person_character_1))

(fn GetPatrolRoute
  (return (Variables|AI|GetPatrolRoute)))

(fn SetMovementSpeed
  (params (Speed :type E_MovementSpeed%20Enum :default "NewEnumerator0"))
  (bind _output_get (Variables|/Script/Engine.CharacterMovementComponent|SetMaxWalkSpeed (Variables|Character|GetCharacterMovement) (Utilities|Select :Index Speed :NewEnumerator0 0.0 :NewEnumerator1 3e+02 :NewEnumerator2 4.5e+02 :NewEnumerator3 6e+02)))
  (return _output_get))