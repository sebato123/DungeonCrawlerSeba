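; One-shot interactable dungeon chest that rewards the player with coins and score when opened.
; Interact accepts only the player character, then sets an Opened flag, snaps the whole actor to a fixed rotation and prints a debug message.
; It calls DropCoins on the caller's BPC_DropSystem component, not one of its own, and adds score through BP_GameMode_Dungeon.
; CanInteract reports true only while the chest is unopened.
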(event EventBeginPlay)

(event Collision|EventActorBeginOverlap
  (params (OtherActor :type Actor%20Object%20Reference)))

(event EventTick
  (params (DeltaSeconds :type Float%20%28single-precision%29)))

(event EventInteract
  (params (Caller :type Actor%20Object%20Reference))
  (bind _asbp_duplicated_third_person_character_1 (Utilities|Casting|CastToBP_DuplicatedThirdPersonCharacter1 Caller))
  (if (not (Variables|Default|GetbOpened%20))
    (Variables|Default|SetbOpened%20 true)
    (Transformation|SetActorRotation "90.000000,0.000000,0.000000")
    (Development|PrintString "abriendo")
    (Default|DropCoins (Actor|GetComponentbyClass _asbp_duplicated_third_person_character_1 "/Game/Assets/3D/Blueprints/BPC_DropSystem.BPC_DropSystem_C"))
    (bind _asbp_game_mode_dungeon (Utilities|Casting|CastToBP_GameMode_Dungeon (Game|GetGameMode)))
    (Default|AddScore _asbp_game_mode_dungeon 20)))

(fn ConstructionScript)

(fn CanInteract
  (params (Caller :type Actor%20Object%20Reference))
  (return (!= (Variables|Default|GetbOpened%20) true)))