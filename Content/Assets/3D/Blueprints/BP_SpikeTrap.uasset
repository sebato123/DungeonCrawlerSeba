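; BP_SpikeTrap is a spike trap that damages the player character on overlap and can be switched on and off through interaction.
; Overlaps cast to BP_DuplicatedThirdPersonCharacter1 and call ReceiveDamage on its health system component.
; Interact toggles the Active state, switching the Box between query-only and no collision and snapping the actor between on and off rotations.
; It starts active, always allows interaction, and prints debug messages throughout.
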(event EventBeginPlay
  (Variables|Default|SetbActive true)
  (Collision|SetCollisionEnabled (Variables|Default|GetBox) "QueryOnly"))

(event Collision|EventActorBeginOverlap
  (params (OtherActor :type Actor%20Object%20Reference))
  (Development|PrintString "Colision")
  (bind _asbp_duplicated_third_person_character_1 (Utilities|Casting|CastToBP_DuplicatedThirdPersonCharacter1 OtherActor))
  (Utilities|IsValid (Actor|GetComponentbyClass _asbp_duplicated_third_person_character_1 "/Game/Assets/3D/Blueprints/BPC_HealthSystemCoponent.BPC_HealthSystemCoponent_C")
    (:Is%20Valid
      (Class|HealthSystemComponent|ReceiveDamage (Actor|GetComponentbyClass _asbp_duplicated_third_person_character_1 "/Game/Assets/3D/Blueprints/BPC_HealthSystemCoponent.BPC_HealthSystemCoponent_C"))
      (Development|PrintString "daño recibido"))
    (:Is%20Not%20Valid
      (Development|PrintString "No es valido"))))

(event EventTick
  (params (DeltaSeconds :type Float%20%28single-precision%29)))

(event EventInteract
  (params (Caller :type Actor%20Object%20Reference))
  (bind _output_get (Variables|Default|SetbActive (not (Variables|Default|GetbActive))))
  (if _output_get
    (Collision|SetCollisionEnabled (Variables|Default|GetBox) "QueryOnly")
    (Development|PrintString "Activada")
    (Transformation|SetActorRotation (Variables|Default|GetRotationOn))
    (else
      (Collision|SetCollisionEnabled (Variables|Default|GetBox) "NoCollision")
      (Development|PrintString "No hay colision")
      (Transformation|SetActorRotation (Variables|Default|GetRotationOff)))))

(fn ConstructionScript)

(fn CanInteract
  (params (Caller :type Actor%20Object%20Reference))
  (return true))