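; Health component that tracks player health, handles damage and healing, and triggers death and defeat in the dungeon game mode.
; MaxHealth serves as current health, clamped on damage or fixed-amount heals and broadcast through EHealthUpdated.
; At zero it sets IsDead, finds the character by class rather than owner, plays death animation and a sound at world origin, disables input and calls HandleDefeat.
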(event Custom|OnDamageReceived_Event
  (bind _output_get (Variables|Default|SetMaxHealth (Math|Float|Clamp(Float) (- (Variables|Default|GetMaxHealth) (Variables|Default|GetDamageAmount)) 0.0 1e+02)))
  (Default|CallEHealthUpdated (Variables|Default|GetMaxHealth) 1e+02)
  (if (== _output_get 0.0)
    (Development|PrintString "Has Muerto")
    (Variables|Default|SetIsDead? true)
    (bind _returnvalue (Actor|GetActorOfClass "/Game/Assets/3D/Blueprints/BP_DuplicatedThirdPersonCharacter1.BP_DuplicatedThirdPersonCharacter1_C"))
    (bind _asbp_duplicated_third_person_character_1 (Utilities|Casting|CastToBP_DuplicatedThirdPersonCharacter1 _returnvalue))
    (Components|Animation|PlayAnimation (Variables|/Script/Engine.Character|GetMesh _asbp_duplicated_third_person_character_1) "/Game/Assets/3D/Animation/AnimationSeq/AN_Death_CharacterDeath.AN_Death_CharacterDeath" false)
    (Audio|PlaySoundatLocation "/Game/Assets/3D/Sounds/SFX/CharacterDie.CharacterDie" "0, 0, 0" "0, 0, 0" 1.0 1.0 0.0 0 0 0 0)
    (Input|DisableInput _asbp_duplicated_third_person_character_1 (Game|GetPlayerController 0))
    (bind _asbp_game_mode_dungeon (Utilities|Casting|CastToBP_GameMode_Dungeon (Game|GetGameMode)))
    (Default|HandleDefeat _asbp_game_mode_dungeon)))

(event Custom|OnHealRecieved
  (Variables|Default|SetMaxHealth (Math|Float|Clamp(Float) (+ (Variables|Default|GetMaxHealth) 5e+01) 0.0 1e+02))
  (Default|CallEHealthUpdated (Variables|Default|GetMaxHealth) 1e+02))

(event EventBeginPlay
  (Variables|Default|SetMaxHealth 1e+02)
  (EventDispatchers|BindEventtoOnDamageReceived (delegate Custom|OnDamageReceived_Event)))