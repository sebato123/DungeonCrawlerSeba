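; BP_Projectile is a projectile actor that damages the player character on overlap.
; On BeginPlay it caches its row from the DT_EnemyStats data table, selected by EnemyRowName.
; Overlapping BP_DuplicatedThirdPersonCharacter1 calls GetHit with that row's DamageDealt, then destroys the projectile and prints a debug message.
; Other overlapping actors are ignored, and the event graph contains no movement logic.
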(event EventBeginPlay
  (bind _returnvalue (Utilities|GetDataTableRow "/Game/Assets/3D/Struct/DT_EnemyStats.DT_EnemyStats" (Variables|Default|GetEnemyRowName))
    (:then
      (if true
        (Variables|Default|SetStats _returnvalue)))))

(event Collision|EventActorBeginOverlap
  (params (OtherActor :type Actor%20Object%20Reference))
  (bind _asbp_duplicated_third_person_character_1 (Utilities|Casting|CastToBP_DuplicatedThirdPersonCharacter1 OtherActor))
  (Default|GetHit _asbp_duplicated_third_person_character_1 (.DamageDealt (Utilities|Struct|BreakST_EnemyStats (Variables|Default|GetStats))))
  (Actor|DestroyActor)
  (Development|PrintString "daño recibido"))

(fn ConstructionScript)