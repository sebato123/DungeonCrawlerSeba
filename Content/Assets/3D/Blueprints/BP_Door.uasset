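; Locked door Blueprint that the player unlocks with a dungeon key and then toggles open and closed.
; On Interact, a locked door casts the caller to the duplicated third-person character and checks its BPC_Inventory for the required item, printing a message if it is missing.
; Once unlocked, each interaction flips the open state and instantly snaps the Anclaje pivot between two relative rotations set at BeginPlay.
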(event EventBeginPlay
  (Variables|Default|SetrotationOpen "0.000000,90.000000,0.000000")
  (Variables|Default|SetrotationClose "0, 0, 0")
  (Variables|Default|SetbLocked true)
  (Variables|Default|SetRequiredItem "DungeonKey"))

(event Collision|EventActorBeginOverlap
  (params (OtherActor :type Actor%20Object%20Reference)))

(event EventTick
  (params (DeltaSeconds :type Float%20%28single-precision%29)))

(event EventInteract
  (params (Caller :type Actor%20Object%20Reference))
  (if (Variables|Default|GetbLocked)
    (bind _asbp_duplicated_third_person_character_1 (Utilities|Casting|CastToBP_DuplicatedThirdPersonCharacter1 Caller))
    (bind _bhasitem (Default|HasItem (Actor|GetComponentbyClass _asbp_duplicated_third_person_character_1 "/Game/Assets/3D/Blueprints/BPC_Inventory.BPC_Inventory_C") (Variables|Default|GetRequiredItem)))
    (if _bhasitem
      (Variables|Default|SetbLocked false)
      (bind _output_get (Variables|Default|SetbOpen (not (Variables|Default|GetbOpen)) :!label _label))
      (if _output_get
        (Development|PrintString "abierta")
        (Transformation|SetRelativeRotation (Variables|Default|GetAnclaje) (Variables|Default|GetrotationOpen) false false)
        (else
          (Development|PrintString "cerrada")
          (Transformation|SetRelativeRotation (Variables|Default|GetAnclaje) (Variables|Default|GetrotationClose) false false)))
      (else
        (Development|PrintString "NO TIENEES LA LLAVEEE")))
    (else
      (goto _label))))

(fn ConstructionScript)

(fn CanInteract
  (params (Caller :type Actor%20Object%20Reference))
  (return true))