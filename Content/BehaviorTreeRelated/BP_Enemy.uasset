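; AI-controlled dungeon enemy that hands its patrol points to BP_EnemyAIController and shows its health on a widget bar.
; HitByPlayer applies fixed damage behind a short timer-reset cooldown.
; A lethal hit awards score through BP_GameMode_Dungeon, stops the behavior logic, unpossesses, ragdolls the mesh and removes the health bar.
; AIHitDetect sphere-traces at the right-hand socket and calls GetHit on the player character.
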(event Custom|Die
  (bind _returnvalue (Pawn|GetController))
  (bind _mesh (Variables|Character|GetMesh))
  (bind _asbp_enemy_aicontroller (Utilities|Casting|CastToBP_EnemyAIController _returnvalue)
    (:then
      (AI|Logic|StopLogic (Variables|/Script/AIModule.AIController|GetBrainComponent _asbp_enemy_aicontroller) "Dead")
      (Pawn|UnPossess _returnvalue)
      (Collision|SetCollisionProfileName _mesh "Ragdoll" true :!class /Script/Engine.PrimitiveComponent)
      (Physics|SetSimulatePhysics _mesh true)
      (Components|DestroyComponent (Variables|Default|GetHealthBarWidget)))
    (:CastFailed
      (Development|PrintString "BP_Enemy - No se obtuvo AI Controller correctamente"))))

(event Custom|ResetDamageFlag
  (Variables|Default|SetCan%20Receive%20Damage true))

(event Custom|HitByPlayer
  ;[0.15 0.15 0.15 0.5] GetHit
  (if (Variables|Default|GetCan%20Receive%20Damage)
    (Variables|Default|SetHealth (- (Variables|Default|GetHealth) 4e+01))
    (if (<= (Variables|Default|GetHealth) 0.0)
      (bind _asbp_game_mode_dungeon (Utilities|Casting|CastToBP_GameMode_Dungeon (Game|GetGameMode))
        (:then
          (Default|AddScore _asbp_game_mode_dungeon 50)
          (Collision|SetCollisionProfileName (Variables|Collision|GetCapsuleComponent) (Utilities|Name|MakeLiteralName "NoCollision") true :!class /Script/Engine.PrimitiveComponent)
          (CallFunction|Die))
        (:CastFailed
          (Development|PrintString "Failed")))
      (else
        (bind _aswbp_enemy_health (Utilities|Casting|CastToWBP_EnemyHealth (UserInterface|GetUserWidgetObject (Variables|Default|GetHealthBarWidget))))
        (Variables|Default|SetAs%20WBP%20Enemy%20Health _aswbp_enemy_health)
        (Variables|/Game/Assets/3D/Widget/WBP_EnemyHealth.WBP_EnemyHealth_C|SetHealth (Variables|Default|GetAs%20WBP%20Enemy%20Health) (/ (Variables|Default|GetHealth) 1e+02))
        (Variables|Default|SetCan%20Receive%20Damage false)
        (Utilities|Time|SetTimerbyFunctionName 0 "ResetDamageFlag" 0.2)))))

(event EventBeginPlay
  (Variables|Default|SetCan%20Receive%20Damage true)
  (bind _asbp_enemy_aicontroller (Utilities|Casting|CastToBP_EnemyAIController (Pawn|GetController)))
  (Variables|/Game/BehaviorTreeRelated/BP_EnemyAIController.BP_EnemyAIController_C|SetPatrolPoints _asbp_enemy_aicontroller (Variables|Default|GetPatrolPoints))
  (Variables|Default|SetHealth 1e+02)
  (bind _aswbp_enemy_health (Utilities|Casting|CastToWBP_EnemyHealth (UserInterface|GetUserWidgetObject (Variables|Default|GetHealthBarWidget))))
  (Variables|Default|SetAs%20WBP%20Enemy%20Health _aswbp_enemy_health)
  (Variables|/Game/Assets/3D/Widget/WBP_EnemyHealth.WBP_EnemyHealth_C|SetHealth (Variables|Default|GetAs%20WBP%20Enemy%20Health) (/ (Variables|Default|GetHealth) 1e+02)))

(event Collision|EventActorBeginOverlap
  (params (OtherActor :type Actor%20Object%20Reference)))

(event EventTick
  (params (DeltaSeconds :type Float%20%28single-precision%29)))

(fn ConstructionScript)

(fn AIHitDetect
  (bind _mesh (Variables|Character|GetMesh))
  (bind _returnvalue (Transformation|GetSocketLocation _mesh "hand_r"))
  (bind _outhit (Collision|SphereTraceForObjects _returnvalue _returnvalue 5e+01 (Utilities|Array|MakeArray "ObjectTypeQuery3") false 0 "ForDuration"))
  (bind _asbp_duplicated_third_person_character_1 (Utilities|Casting|CastToBP_DuplicatedThirdPersonCharacter1 (.HitActor (Collision|BreakHitResult _outhit))))
  (Default|GetHit _asbp_duplicated_third_person_character_1))