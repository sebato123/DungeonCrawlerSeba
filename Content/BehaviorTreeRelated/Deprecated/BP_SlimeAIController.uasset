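; Deprecated AI controller for the slime enemy, which starts its blackboard and behavior tree on BeginPlay.
; AI perception updates store the player character as TargetActor and branch on sense class, printing debug messages.
; Sight sets HasLOS and resets LostSightTime, hearing changes nothing further, and any other sense clears HasLOS.
; It never checks whether sensing succeeded, so losing sight also takes the sight branch.
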(event OnTargetPerceptionUpdated(AIPerception)
  (params (Actor :type Actor%20Object%20Reference) (Stimulus :type AI%20Stimulus%20Structure))
  (bind _blackboardcomp (Variables|Default|GetBlackboardComp))
  (bind _returnvalue (Class|AIPerceptionSystem|GetSenseClassforStimulus Stimulus))
  (bind _asbp_duplicated_third_person_character_1 (Utilities|Casting|CastToBP_DuplicatedThirdPersonCharacter1 Actor)
    (:then
      (AI|Components|Blackboard|SetValueasObject _blackboardcomp (Utilities|Name|MakeLiteralName "TargetActor") _asbp_duplicated_third_person_character_1)
      (if (== _returnvalue "/Script/AIModule.AISense_Sight")
        (AI|Components|Blackboard|SetValueasBool _blackboardcomp (Utilities|Name|MakeLiteralName "HasLOS") true)
        (AI|Components|Blackboard|SetValueasFloat _blackboardcomp (Utilities|Name|MakeLiteralName "LostSightTime") 0.0)
        (Development|PrintString "Seen Player")
        (elif (== _returnvalue "/Script/AIModule.AISense_Hearing")
          (Development|PrintString "Heard Player")
          (else
            (AI|Components|Blackboard|SetValueasBool _blackboardcomp (Utilities|Name|MakeLiteralName "HasLOS") false)
            (Development|PrintString " Lost LOS")))))
    (:CastFailed
      (Development|PrintString "No se encontró al jugador (Slime)"))))

(event EventBeginPlay
  (bind _blackboardcomponent (Class|AIController|UseBlackboard "/Game/BehaviorTreeRelated/Deprecated/BB_Slime.BB_Slime"))
  (AI|RunBehaviorTree "/Game/BehaviorTreeRelated/Deprecated/BT_Slime.BT_Slime")
  (Variables|Default|SetBlackboardComp _blackboardcomponent))

(fn ConstructionScript)