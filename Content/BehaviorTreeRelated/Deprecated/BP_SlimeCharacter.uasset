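; Deprecated slime character that performs a cooldown-gated leap attack toward a target actor.
; DoLeapTo stops movement, launches the slime toward the target and opens the AttackHit collision window briefly.
; The window closes after a short delay or on landing, which also restarts the cooldown.
; The hit overlap applies no effect yet, and SetMoveSpeed adjusts walk speed.
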(event OnComponentBeginOverlap(AttackHit)
  (params (OverlappedComponent :type Primitive%20Component%20Object%20Reference) (OtherActor :type Actor%20Object%20Reference) (OtherComp :type Primitive%20Component%20Object%20Reference) (OtherBodyIndex :type Integer) (bFromSweep :type Boolean) (SweepResult :type Hit%20Result%20Structure%20%28by%20ref%29))
  (if (Variables|Default|GetAttackWindowActive)
    _))

(event Custom|DoLeapTo
  (params (Target :type Actor%20Object%20Reference))
  (if (not (Variables|Default|GetisLeaping))
    (if (> (- (Utilities|Time|GetGameTimeinSeconds) (Variables|Default|GetLastLeapTime)) (Variables|Default|GetLeapCooldown))
      (Components|Movement|StopMovementImmediately (Variables|Character|GetCharacterMovement))
      (Character|LaunchCharacter (+ (* (Math|Vector|Normalize (- (Transformation|GetActorLocation Target) (Transformation|GetActorLocation self))) (Variables|Default|GetLeapStrengthXY)) (Variables|Default|GetLeapStrengthZ)) true true)
      (Variables|Default|SetisLeaping true)
      (CallFunction|EnableAttackWindow true)
      (Utilities|FlowControl|Delay 0.3)
      (CallFunction|EnableAttackWindow false)
      (Variables|Default|SetisLeaping false))))

(event EventBeginPlay
  (Development|PrintString "SlimeReady"))

(event EventOnLanded
  (params (Hit :type Hit%20Result%20Structure%20%28by%20ref%29))
  (Variables|Default|SetisLeaping false)
  (CallFunction|EnableAttackWindow false)
  (Variables|Default|SetLastLeapTime (Utilities|Time|GetGameTimeinSeconds))
  (Development|PrintString "Landed"))

(fn ConstructionScript)

(fn EnableAttackWindow
  (params (bEnable :type Boolean))
  (if bEnable
    (Collision|SetCollisionEnabled (Variables|Default|GetAttackHit) "QueryOnly")
    (else
      (Collision|SetCollisionEnabled (Variables|Default|GetAttackHit) "NoCollision")))
  (Variables|Default|SetAttackWindowActive bEnable))

(fn SetMoveSpeed
  (params (NewSpeed :type Float%20%28double-precision%29))
  (Variables|/Script/Engine.CharacterMovementComponent|SetMaxWalkSpeed (Variables|Character|GetCharacterMovement self) NewSpeed))