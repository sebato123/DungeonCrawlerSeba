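; Enemy AI controller that runs BT_Enemy and feeds it patrol and perception data through the blackboard.
; On BeginPlay it seeds PatrolTarget with the first patrol point, if any exist.
; Perception updates store sighted actors as TargetActor, while other successful stimuli, treated as hearing, set LastHeardLocation.
; A failed stimulus from the current target clears TargetActor, whichever sense reported it, and debug prints trace these changes.
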(event OnTargetPerceptionUpdated(AIPerception)
  (params (Actor :type Actor%20Object%20Reference) (Stimulus :type AI%20Stimulus%20Structure))
  (bind (_age _expirationage _strength _stimuluslocation _receiverlocation _tag _bsuccessfullysensed) (Utilities|Struct|BreakAIStimulus Stimulus))
  (bind _returnvalue (AI|GetBlackboard 0))
  (bind _returnvalue_2 (AI|GetBlackboard 0))
  (bind _returnvalue_3 (Utilities|Name|MakeLiteralName "TargetActor"))
  ;[0.15 0.15 0.15 0.5] Verificamos si fue verificado o no, y por cual estimulo
  (bind _returnvalue_4 (Class|AIPerceptionSystem|GetSenseClassforStimulus Stimulus))
  (bind _output_get (Variables|Default|SetDetectedBySight (== _returnvalue_4 "/Script/AIModule.AISense_Sight")))
  (if _bsuccessfullysensed
    ;[0.15 0.15 0.15 0.5] Si fue detectado por vista o oido
    (if _output_get
      (AI|Components|Blackboard|SetValueasObject _returnvalue (Utilities|Name|MakeLiteralName "TargetActor") Actor)
      (Development|PrintString "AIController - Se ha visto y establecido jugador")
      (else
        (AI|Components|Blackboard|SetValueasVector _returnvalue (Utilities|Name|MakeLiteralName "LastHeardLocation") _stimuluslocation)
        (Development|PrintString "AIController - Se escucho jugador, LastHeardLocation Establecido")))
    (elif (== (AI|Components|Blackboard|GetValueasObject _returnvalue_2 _returnvalue_3) Actor)
      (AI|Components|Blackboard|ClearValue _returnvalue_2 _returnvalue_3)
      (Development|PrintString "AIController - Se perdio al jugador, limpiando TargetActor"))))

(event EventBeginPlay
  (AI|RunBehaviorTree "/Game/BehaviorTreeRelated/BT_Enemy.BT_Enemy")
  (if (> (Utilities|Array|Length (Variables|Default|GetPatrolPoints)) 0)
    (AI|Components|Blackboard|SetValueasObject (AI|GetBlackboard 0) (Utilities|Name|MakeLiteralName "PatrolTarget") (Utilities|Array|Get(acopy) (Variables|Default|GetPatrolPoints)))))

(fn ConstructionScript)